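; BP_AT is the Alan Turing character Blueprint that shows a line-by-line dialogue on screen.
; Each ATTalk call increments TalkIndex and writes that Dialog entry into the WBP_AT_Dialog widget's text.
; The widget is created for player 0 if no valid one exists, and is removed from the screen once the index passes the last line.
; TalkIndex is never reset in this graph.
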(event EventATTalk
  (Math|Integer|IncrementInt (Variables|Default|GetTalkIndex)
    (:%20%20
      (if (< (Variables|Default|GetTalkIndex) (Utilities|Array|Length (Variables|Default|GetDialog)))
        (Variables|Default|GetUI
          (:then
            _)
          (:else
            (bind _returnvalue (UserInterface|CreateWidget "/Game/Characters/AlanTuring/WBP_AT_Dialog.WBP_AT_Dialog_C" (Game|GetPlayerController 0)))
            (bind _output_get (Variables|Default|SetUI _returnvalue))
            (UserInterface|Viewport|AddtoViewport _output_get 0)))
        (Rendering|Components|TextRender|SetText (Variables|/Game/Characters/AlanTuring/WBP_AT_Dialog.WBP_AT_Dialog_C|GetTalkTextUI (Variables|Default|GetUI)) (Utilities|Text|ToText(String) (Utilities|Array|Get(acopy) (Variables|Default|GetDialog) (Variables|Default|GetTalkIndex))))
        (else
          (Widget|RemovefromParent (Variables|Default|GetUI)))))))

(fn ConstructionScript)