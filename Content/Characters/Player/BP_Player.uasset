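; Player character Blueprint that handles movement and talking to nearby NPCs.
; BeginPlay adds the Enhanced Input mapping context; move input drives movement along fixed world X and inverted Y axes, storing direction and held state.
; Three separate E-key handlers each find overlapping BP_AT, BP_WN or BP_AL actors and call that type's own dialog interface message.
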(event Input|EnhancedActionEvents|EnhancedInputActionIA_PlayerMove
  (params (ActionValue :type Vector%202D%20Structure) (ElapsedSeconds :type Float%20%28double-precision%29) (TriggeredSeconds :type Float%20%28double-precision%29) (InputAction :type Input%20Action%20Object%20Reference :default "/Game/Characters/Player/Input/IA_PlayerMove.IA_PlayerMove"))
  ;[1 1 1] Player Movement
  (:Triggered
    (Pawn|Input|AddMovementInput "1.000000,0.000000,0.000000" (.x ActionValue) false) ; Left/Right
    (Pawn|Input|AddMovementInput "0.000000,-1.000000,0.000000" (.y ActionValue) false) ; Up/Down
    (Variables|Default|SetDirectionality (Math|Vector2D|MakeVector2D (.x ActionValue) (.y ActionValue))))
  (:Started
    (Variables|Default|SetIsHoldingMove true))
  (:Completed
    (Variables|Default|SetIsHoldingMove false)))

(event EventBeginPlay
  ;[1 1 1] Player Animation Stuff??
  (bind _asplayer_controller (Utilities|Casting|CastToPlayerController (Pawn|GetController)))
  (Input|AddMappingContext (PlayerController|LocalPlayerSubsystems|GetEnhancedInputLocalPlayerSubsystem _asplayer_controller) "/Game/Characters/Player/Input/IMC_PlayerMove.IMC_PlayerMove" 0 "(bIgnoreAllPressedKeysUntilRelease=True,bForceImmediately=False,bNotifyUserSettings=False)"))

(event Collision|EventActorBeginOverlap
  (params (OtherActor :type Actor%20Object%20Reference)))

(event EventTick
  (params (DeltaSeconds :type Float%20%28single-precision%29)))

(event Input|KeyboardEvents|E
  (params (Key :type Key%20Structure :default "None"))
  (:Pressed
    (for _array_element (Collision|GetOverlappingActors "/Game/Characters/OtherNPCs/AudreLorde/BP_AL.BP_AL_C" :!class /Script/Engine.Actor)
      (if (Utilities|DoesObjectImplementInterface _array_element "/Game/Characters/OtherNPCs/AudreLorde/BPI_AL_Talk.BPI_AL_Talk_C")
        (Class|BPIALTalk|ALTalk(Message) _array_element)))))

(event Input|KeyboardEvents|E
  (params (Key :type Key%20Structure :default "None"))
  (:Pressed
    (for _array_element (Collision|GetOverlappingActors "/Game/Characters/OtherNPCs/WilliNinja/BP_WN.BP_WN_C" :!class /Script/Engine.Actor)
      (if (Utilities|DoesObjectImplementInterface _array_element "/Game/Characters/OtherNPCs/WilliNinja/BPI_WN_Talk.BPI_WN_Talk_C")
        (Class|BPIWNTalk|WNTalk(Message) _array_element)))))

(event Input|KeyboardEvents|E
  (params (Key :type Key%20Structure :default "None"))
  (:Pressed
    (for _array_element (Collision|GetOverlappingActors "/Game/Characters/AlanTuring/BP_AT.BP_AT_C" :!class /Script/Engine.Actor)
      (if (Utilities|DoesObjectImplementInterface _array_element "/Game/Characters/AlanTuring/BPI_AT_Dialog.BPI_AT_Dialog_C")
        (Class|BPIATDialog|ATTalk(Message) _array_element)))))

(fn ConstructionScript)